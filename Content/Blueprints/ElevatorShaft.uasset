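; Elevator shaft Blueprint with two sliding doors that open on the Interact input and close when a collider overlap ends.
; Overlapping either door collider enables player input, and separate Interact events play the left and right timelines, whose curves drive each door's relative location.
; Ending an overlap reverses that door's timeline.
; The DisableInput calls are unconnected, so input stays enabled and Interact is not tied to a specific door.
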(event `self.DoorCollider2.OnComponentBeginOverlap`
  (params (OverlappedComponent :type "PrimitiveComponent Object Reference") (OtherActor :type "Actor Object Reference") (OtherComp :type "PrimitiveComponent Object Reference") (OtherBodyIndex :type Integer) (bFromSweep :type Boolean) (SweepResult :type "HitResult Structure (by ref)"))
  ;[1 1 1] get input for door 2
  (`self.EnableInput` (`GameplayStatics.GetPlayerController` 0)))

(event `self.DoorCollider1.OnComponentBeginOverlap`
  (params (OverlappedComponent :type "PrimitiveComponent Object Reference") (OtherActor :type "Actor Object Reference") (OtherComp :type "PrimitiveComponent Object Reference") (OtherBodyIndex :type Integer) (bFromSweep :type Boolean) (SweepResult :type "HitResult Structure (by ref)"))
  ;[1 1 1] Check for input on door 1
  (`self.EnableInput` (`GameplayStatics.GetPlayerController` 0)))

(event `self.DoorCollider2.OnComponentEndOverlap`
  (params (OverlappedComponent :type "PrimitiveComponent Object Reference") (OtherActor :type "Actor Object Reference") (OtherComp :type "PrimitiveComponent Object Reference") (OtherBodyIndex :type Integer))
  ;[1 1 1] get input for door 2
  ;[1 1 1] door 2 open
  (bind (_direction _x_curve2 _y_curve _z_curve) (`Timeline|DoorOpenRight` :!via `Reverse` :!label _label)
    (:`Update`
      (`SceneComponent.K2_SetRelativeLocation` (`self.door2`) (`KismetMathLibrary.MakeVector` _x_curve2 _y_curve _z_curve) false false))))

(event `self.DoorCollider1.OnComponentEndOverlap`
  (params (OverlappedComponent :type "PrimitiveComponent Object Reference") (OtherActor :type "Actor Object Reference") (OtherComp :type "PrimitiveComponent Object Reference") (OtherBodyIndex :type Integer))
  ;[1 1 1] Check for input on door 1
  ;[1 1 1] door 1 open
  (bind (_direction _x_curve _z_curve _y_curve) (`Timeline|DoorOpenLeft` :!via `Reverse` :!label _label_2)
    (:`Update`
      (`SceneComponent.K2_SetRelativeLocation` (`self.Door1`) (`KismetMathLibrary.MakeVector` _x_curve _y_curve _z_curve) false false))))

(event `InputAction|Interact`
  (params (Key :type "Key Structure"))
  ;[1 1 1] door 1 open
  (:`Pressed`
    (goto _label_2)))

(event `InputAction|Interact`
  (params (Key :type "Key Structure"))
  ;[1 1 1] door 2 open
  (:`Pressed`
    (goto _label)))

(fn `UserConstructionScript`)