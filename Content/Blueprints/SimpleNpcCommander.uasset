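; Simple NPC commander that shows dialogue and updates the quest text when any actor overlaps it.
; Begin overlap creates the dialog widget with MyText, or removes it if one is already flagged open; end overlap also removes it.
; Each widget creation flips QuestDoor, alternating the ThirdPersonGameMode Quest string between finding a quest and talking to the commander.
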(event `self.ReceiveActorEndOverlap`
  (params (OtherActor :type "Actor Object Reference"))
  (`Widget.RemoveFromParent` (`self.DialogWigit`) :!label _label)
  (set `self.DialogWigit` null)
  (set `self.dialogCheck` false))

(event `self.ReceiveActorBeginOverlap`
  (params (OtherActor :type "Actor Object Reference"))
  (`|ExecutionSequence`
    (:`then_0`
      (if (`self.dialogCheck`)
        (goto _label)
        (else
          (bind _returnvalue (`|CreateWidget` "/Game/DialogWigit.DialogWigit_C" (`GameplayStatics.GetPlayerController` 0)))
          (bind _output_get (set `self.DialogWigit` _returnvalue))
          (set `self.dialogCheck` true)
          (`UserWidget.AddToViewport` _output_get 0)
          (set `/Game/DialogWigit.DialogText` (`self.MyText`) (`self.DialogWigit`))
          (if (`self.QuestDoor`)
            (bind _asthird_person_game_mode (cast `/Game/ThirdPersonGameMode` (`GameplayStatics.GetGameMode`)))
            (set `/Game/ThirdPersonGameMode.Quest` "Find a quest" _asthird_person_game_mode)
            (set `self.QuestDoor` false)
            (else
              (bind _asthird_person_game_mode_2 (cast `/Game/ThirdPersonGameMode` (`GameplayStatics.GetGameMode`)))
              (set `/Game/ThirdPersonGameMode.Quest` "Talk to the commander" _asthird_person_game_mode_2)
              (set `self.QuestDoor` true))))))))

(fn `UserConstructionScript`)