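; GateDoor2 is a key card gate that slides a door vertically through the DoorOpen timeline.
; Overlapping the SpaceToClick component enables player input, and Interact plays the timeline if the game mode's KeyCard count is at least one, resetting it to zero.
; Ending the overlap reverses the timeline to close the door.
; The DisableInput call is unconnected, so input stays enabled after leaving.
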(event `self.SpaceToClick.OnComponentBeginOverlap`
  (params (OverlappedComponent :type "PrimitiveComponent Object Reference") (OtherActor :type "Actor Object Reference") (OtherComp :type "PrimitiveComponent Object Reference") (OtherBodyIndex :type Integer) (bFromSweep :type Boolean) (SweepResult :type "HitResult Structure (by ref)"))
  ;[1 1 1] Listen for input
  (`self.EnableInput` (`GameplayStatics.GetPlayerController` 0)))

(event `self.SpaceToClick.OnComponentEndOverlap`
  (params (OverlappedComponent :type "PrimitiveComponent Object Reference") (OtherActor :type "Actor Object Reference") (OtherComp :type "PrimitiveComponent Object Reference") (OtherBodyIndex :type Integer))
  ;[1 1 1] Listen for input
  (bind (_direction _z_pos) (`Timeline|DoorOpen` :!via `Reverse` :!label _label)
    (:`Update`
      (`SceneComponent.K2_SetRelativeLocation` (`self.door`) (`KismetMathLibrary.MakeVector` 0.0 0.0 _z_pos) false false))))

(event `InputAction|Interact`
  (params (Key :type "Key Structure"))
  (:`Pressed`
    (bind _asthird_person_game_mode (cast `/Game/StarterContent/ThirdPersonBP/Blueprints/ThirdPersonGameMode` (`GameplayStatics.GetGameMode`)))
    (if (>= (`/Game/StarterContent/ThirdPersonBP/Blueprints/ThirdPersonGameMode.KeyCard` _asthird_person_game_mode) 1)
      (set `/Game/StarterContent/ThirdPersonBP/Blueprints/ThirdPersonGameMode.KeyCard` 0 _asthird_person_game_mode)
      (goto _label))))

(fn `UserConstructionScript`)