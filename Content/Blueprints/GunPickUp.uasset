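; GunPickUp is an overlap pickup that, despite its name, grants one experience point and then destroys itself.
; Any overlap with its Sphere component triggers it, with no check on the overlapping actor.
; It updates progression directly on ThirdPersonGameMode, raising Level, resetting Experience and doubling MaxExperience when the threshold is reached.
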(event `self.Sphere.OnComponentBeginOverlap`
  (params (OverlappedComponent :type "PrimitiveComponent Object Reference") (OtherActor :type "Actor Object Reference") (OtherComp :type "PrimitiveComponent Object Reference") (OtherBodyIndex :type Integer) (bFromSweep :type Boolean) (SweepResult :type "HitResult Structure (by ref)"))
  (bind _asthird_person_game_mode (cast `/Game/ThirdPersonGameMode` (`GameplayStatics.GetGameMode`)))
  (bind _output_get (set `/Game/ThirdPersonGameMode.Experience` (+ (`/Game/ThirdPersonGameMode.Experience` _asthird_person_game_mode) 1) _asthird_person_game_mode))
  (if (>= _output_get (`/Game/ThirdPersonGameMode.MaxExperience` _asthird_person_game_mode))
    (set `/Game/ThirdPersonGameMode.Level` (+ (`/Game/ThirdPersonGameMode.Level` _asthird_person_game_mode) 1) _asthird_person_game_mode)
    (set `/Game/ThirdPersonGameMode.Experience` 0 _asthird_person_game_mode)
    (set `/Game/ThirdPersonGameMode.MaxExperience` (* (`/Game/ThirdPersonGameMode.MaxExperience` _asthird_person_game_mode) 2) _asthird_person_game_mode))
  (`self.K2_DestroyActor`))

(fn `UserConstructionScript`)