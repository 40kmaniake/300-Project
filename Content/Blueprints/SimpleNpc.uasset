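; SimpleNpc is an NPC actor that shows a dialog widget when another actor overlaps it.
; Begin overlap creates the widget for player 0, adds it to the viewport and fills its text from MyText.
; End overlap, or a begin overlap while DialogCheck is set, removes the widget and clears the flag.
; The overlapping actor is not filtered.
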(event `self.ReceiveActorEndOverlap`
  (params (OtherActor :type "Actor Object Reference"))
  (`Widget.RemoveFromParent` (`self.DialogWigit`) :!label _label)
  (set `self.DialogWigit` null)
  (set `self.dialogCheck` false))

(event `self.ReceiveActorBeginOverlap`
  (params (OtherActor :type "Actor Object Reference"))
  (if (`self.dialogCheck`)
    (goto _label)
    (else
      (bind _returnvalue (`|CreateWidget` "/Game/DialogWigit.DialogWigit_C" (`GameplayStatics.GetPlayerController` 0)))
      (bind _output_get (set `self.DialogWigit` _returnvalue))
      (set `self.dialogCheck` true)
      (`UserWidget.AddToViewport` _output_get 0)
      (set `/Game/DialogWigit.DialogText` (`self.MyText`) (`self.DialogWigit`)))))

(fn `UserConstructionScript`)